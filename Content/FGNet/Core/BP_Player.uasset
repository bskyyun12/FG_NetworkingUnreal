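; BP_Player is a networking test player that exercises the FGReplicator system with a smoothed value and shows its network role on a widget.
; On BeginPlay it registers an FGValueReplicator named "SmoothValue" and writes the local role into the WBP_Role widget.
; Tick prints the replicated value, and pressing B raises it by a random amount.
; Rocket count changes are forwarded to the same widget.
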(event `self.ReceiveBeginPlay`
  (`|ExecutionSequence`
    (:`then_0`
      (bind _returnvalue (`FGReplicatorComponent.AddReplicatorByClass` (`self.FGReplicator`) "/Script/FGNet.FGValueReplicator" "SmoothValue"))
      (bind _asfgvalue_replicator (cast `FGValueReplicator` _returnvalue))
      (set `self.ValueReplicator` _asfgvalue_replicator))
    (:`then_1`
      (bind _aswbp_role (cast `/Game/FGNet/UI/WBP_Role` (`WidgetComponent.GetUserWidgetObject` (`self.Widget_Role`))))
      (`/Game/FGNet/UI/WBP_Role.SetLocalText` _aswbp_role (`self.GetLocalRoleText`)))))

(event `self.BP_OnNumRocketsChanged`
  (params (NewNumRockets :type Integer))
  (bind _aswbp_role (cast `/Game/FGNet/UI/WBP_Role` (`WidgetComponent.GetUserWidgetObject` (`self.Widget_Role`))))
  (`/Game/FGNet/UI/WBP_Role.SetNumRockets` _aswbp_role NewNumRockets))

(event `self.ReceiveTick`
  (params (DeltaSeconds :type "Float (single-precision)"))
  (`KismetSystemLibrary.PrintString` (`KismetStringLibrary.Conv_DoubleToString` (`FGValueReplicator.GetValue` (`self.ValueReplicator`))) true true (struct :`G` 0.66 :`B` 1.0 :`A` 1.0) DeltaSeconds))

(event `Key|B`
  (params (Key :type "Key Structure"))
  (bind _valuereplicator (`self.ValueReplicator`))
  (:`Pressed`
    (`FGValueReplicator.SetValue` _valuereplicator (+ (`FGValueReplicator.GetValue` _valuereplicator) (`KismetMathLibrary.RandomFloatInRange` 10.0 200.0)))))

(fn `GetLocalRoleText`
  (returns (ReturnValue :type Text))
  (return (`KismetTextLibrary.Conv_StringToText` (`|GetEnumeratorNameAsString` (`self.GetLocalRole`)))))

(fn `GetRemoteRoleText`
  (returns (ReturnValue :type Text))
  (return (`KismetTextLibrary.Conv_StringToText` (`|GetEnumeratorNameAsString` (`self.GetRemoteRole`)))))

(fn `UserConstructionScript`)